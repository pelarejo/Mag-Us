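; Player character Blueprint that recognizes Leap Motion hand gestures.
; On BeginPlay it enables swipe, circle and key tap detection on its Leap controller.
; When a gesture is detected, it switches on the type, gets a name string from a small helper function, passes it to GetGestureType and prints a debug message.
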(event EventBeginPlay
  (bind _leapcontroller1 (Variables|Default|GetLeapController1))
  (Class|LeapController|EnableGesture _leapcontroller1 "GESTURE_TYPE_SWIPE" true)
  (Class|LeapController|EnableGesture _leapcontroller1 "GESTURE_TYPE_CIRCLE" true)
  (Class|LeapController|EnableGesture _leapcontroller1 "GESTURE_TYPE_KEY_TAP" true))

(event EventGestureDetected
  (params (gesture :type Leap%20Gesture%20Object%20Reference))
  (switch Utilities|FlowControl|Switch|SwitchonLeapGestureType (Variables|/Script/LeapMotion.LeapGesture|GetType gesture)
    (:GESTURE_TYPE_SWIPE
      (bind _swipe (CallFunction|SwipetoString))
      (Class|MagUsPlayerCharacter|GetGestureType _swipe)
      (Development|PrintString 0 "Swipe"))
    (:GESTURE_TYPE_CIRCLE
      (bind _ret (CallFunction|CircletoString))
      (Class|MagUsPlayerCharacter|GetGestureType _ret)
      (Development|PrintString 0 "Circle" true true "(R=1.000000,G=0.093488,B=0.000000,A=1.000000)"))
    (:GESTURE_TYPE_KEY_TAP
      (bind _keytap (CallFunction|KeyTaptoString))
      (Class|MagUsPlayerCharacter|GetGestureType _keytap)
      (Development|PrintString 0 "Key Tap" true true "(R=0.354877,G=1.000000,B=0.000000,A=1.000000)"))))

(fn ConstructionScript)

(fn CircletoString
  (return "Circle"))

(fn SwipetoString
  (return "Swipe"))

(fn KeyTaptoString
  (return "KeyTap"))