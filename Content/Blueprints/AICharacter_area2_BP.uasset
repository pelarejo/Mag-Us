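; AI character Blueprint for an enemy-attacking unit that uses a goblin sword-slash animation.
; When an enemy is found, it waits its fire rate with slight random jitter, plays the slash, then calls OnFire half a second later; losing the enemy does nothing.
; Destruction also destroys every actor in its Debuffs list.
; MoveForward and MoveRight axis inputs drive movement relative to control yaw.
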(event Custom|Enemy%20Found_Event
  (Utilities|FlowControl|Delay (+ (Variables|Default|GetFireRate) (Math|Random|RandomFloatinRange -0.3 0.3)))
  (Components|Animation|PlayAnimation "/Game/MixamoAnimPack/Mixamo_Goblin/Anims/Mixamo_Goblin_Sword_slash.Mixamo_Goblin_Sword_slash" false)
  (Utilities|FlowControl|Delay 0.5)
  (Class|MagUsAICharacter|OnFire self))

(event Custom|Enemy%20Lost_Event)

(event EventDestroyed
  (for _array_element (Variables|Default|GetDebuffs)
    (Actor|DestroyActor _array_element)))

(event Input|AxisEvents|InputAxisMoveForward
  (params (AxisValue :type Float%20%28single-precision%29))
  (Pawn|Input|AddMovementInput (Math|Vector|GetForwardVector (Class|KismetMathLibrary|MakeRot 0.0 (.Yaw (Class|KismetMathLibrary|BreakRot (Pawn|GetControlRotation :!class /Script/Engine.Pawn))) 0.0)) AxisValue false))

(event Input|AxisEvents|InputAxisMoveRight
  (params (AxisValue :type Float%20%28single-precision%29))
  (Pawn|Input|AddMovementInput (Math|Vector|GetRightVector (Class|KismetMathLibrary|MakeRot 0.0 (.Yaw (Class|KismetMathLibrary|BreakRot (Pawn|GetControlRotation :!class /Script/Engine.Pawn))) 0.0)) AxisValue false))

(fn ConstructionScript)