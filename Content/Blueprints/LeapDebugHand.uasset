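; LeapDebugHand is a debug-drawing helper actor that visualizes Leap Motion hand, finger and arm tracking data.
; Finger bone centers, wrist and elbow become debug spheres, with positions rotated by actor rotation, scaled and offset to actor location.
; Palm and arm orientations become arrows tipped with boxes, offset only by actor location, ignoring its rotation.
; The file contains no events, and nothing in it calls the top-level Debug functions.
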(fn ConstructionScript)

(fn DebugSphereatActor
  (params (Location :type Vector) (Scale :type Float%20%28single-precision%29) (Radius :type Float%20%28single-precision%29))
  (Rendering|Debug|DrawDebugSphere 0 (+ (* (Math|Vector|RotateVector Location (Transformation|GetActorRotation)) Scale) (Transformation|GetActorLocation)) Radius 12 "(R=0.000000,G=0.000000,B=0.000000,A=1.000000)"))

(fn DebugFinger
  (params (Finger :type Leap%20Finger%20Object%20Reference) (Scale :type Float%20%28single-precision%29))
  (CallFunction|DebugSphereatActor (Variables|/Script/LeapMotion.LeapBone|GetCenter (Variables|/Script/LeapMotion.LeapFinger|GetDistal Finger)) Scale Scale)
  (CallFunction|DebugSphereatActor (Variables|/Script/LeapMotion.LeapBone|GetCenter (Variables|/Script/LeapMotion.LeapFinger|GetIntermediate Finger)) Scale Scale)
  (CallFunction|DebugSphereatActor (Variables|/Script/LeapMotion.LeapBone|GetCenter (Variables|/Script/LeapMotion.LeapFinger|GetProximal Finger)) Scale Scale)
  (CallFunction|DebugSphereatActor (Variables|/Script/LeapMotion.LeapBone|GetCenter (Variables|/Script/LeapMotion.LeapFinger|GetMetacarpal Finger)) Scale Scale))

(fn DebugHand
  (params (Hand :type Leap%20Hand%20Object%20Reference) (Scale :type Float%20%28single-precision%29))
  (bind _arm (Variables|/Script/LeapMotion.LeapHand|GetArm Hand))
  (LocalVariables|SetElbowRadius 4.0)
  (LocalVariables|SetWrist%20Radius 2.0)
  (CallFunction|DebugSphereatActor (Variables|/Script/LeapMotion.LeapArm|GetWristPosition _arm) Scale (LocalVariables|GetWrist%20Radius))
  (CallFunction|DebugSphereatActor (Variables|/Script/LeapMotion.LeapArm|GetElbowPosition _arm) Scale (LocalVariables|GetElbowRadius)))

(fn DebugOrientation
  (params (Orientation :type Rotator) (At :type Vector) (Scale :type Float%20%28single-precision%29))
  (bind _returnvalue (Math|Vector|GetForwardVector Orientation))
  (bind _returnvalue_2 (* _returnvalue Scale))
  (bind _returnvalue_3 (+ At _returnvalue_2))
  (Rendering|Debug|DrawDebugArrow :LineStart At :LineEnd _returnvalue_3 :ArrowSize 5.0)
  (Rendering|Debug|DrawDebugBox :Center _returnvalue_3 :Extent "10.000000,10.000000,10.000000" :Rotation Orientation))

(fn DebugHandOrientation
  (params (Hand :type Leap%20Hand%20Object%20Reference))
  (CallFunction|DebugOrientation (Variables|/Script/LeapMotion.LeapHand|GetPalmOrientation Hand) (+ (Transformation|GetActorLocation) (Variables|/Script/LeapMotion.LeapHand|GetPalmPosition Hand)) 5e+01))

(fn DebugArmOrientation
  (params (Arm :type Leap%20Arm%20Object%20Reference))
  (CallFunction|DebugOrientation (Math|Conversions|RotationFromXVector (Variables|/Script/LeapMotion.LeapArm|GetDirection Arm)) (+ (Transformation|GetActorLocation) (Variables|/Script/LeapMotion.LeapArm|GetElbowPosition Arm)) 5e+01))